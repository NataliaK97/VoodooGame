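; Behavior tree task that moves the ghost AI's pawn toward the actor stored in a blackboard key.
; It casts the owner to BP_Ghost_AIController and caches that reference for later runs.
; AI MoveTo follows the TargetToFollow actor with a small acceptance radius.
; The task finishes only when the move succeeds; a failed move or failed cast never calls FinishExecute.
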(event EventReceiveExecute
  (params (OwnerActor :type Actor%20Object%20Reference))
  (if (!= (Variables|Default|GetAIController_Ref) 0)
    _
    (else
      (bind _asbp_ghost_aicontroller (Utilities|Casting|CastToBP_Ghost_AIController OwnerActor))
      (Variables|Default|SetAIController_Ref _asbp_ghost_aicontroller)))
  (AI|AIMoveTo (Pawn|GetControlledPawn (Variables|Default|GetAIController_Ref)) "0, 0, 0" (AI|BehaviorTree|GetBlackboardValueasActor (Variables|Default|GetTargetToFollow)) 5e+01 false
    (:OnSuccess
      (AI|BehaviorTree|FinishExecute true))))