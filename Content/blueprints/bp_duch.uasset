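; Ghost actor (duch) that stays invisible until the player character's cemetery task flag is set.
; BeginPlay hides its Cone and PSteamLit components.
; Tick polls WyswietlZadanieCmentarz on the player's ThirdPersonCharacter and shows both components while it is true, with no logic to hide them again.
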(event EventBeginPlay
  (Rendering|SetVisibility (Variables|Default|GetCone) false false))

(event Collision|EventActorBeginOverlap
  (params (OtherActor :type Actor%20Object%20Reference)))

(event EventTick
  (params (DeltaSeconds :type Float%20%28single-precision%29))
  (bind _asthird_person_character (Utilities|Casting|CastToThirdPersonCharacter (Game|Player|GetPlayerPawn 0)))
  (if (Variables|/Game/ThirdPersonBP/Blueprints/ThirdPersonCharacter.ThirdPersonCharacter_C|GetWyswietlZadanieCmentarz _asthird_person_character)
    (Rendering|SetVisibility (Variables|Default|GetCone) true false)))

(fn ConstructionScript)