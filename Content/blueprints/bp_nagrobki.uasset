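; Gravestone actor (nagrobki) that randomizes its look on spawn and reacts when the player enters its collision volume.
; BeginPlay keeps one of six headstone meshes, destroys the rest, picks one of two materials and, for the first four, reveals a random candle, flame and wax layout.
; Overlap rerolls four Los values on the character, shows the Ul_nagrobki widget and flags Regina's AnimBP; leaving reverts widget and flag.
; Tick clears IsPPresed while overlapping.
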(event OnComponentBeginOverlap(collision)
  (params (OverlappedComponent :type Primitive%20Component%20Object%20Reference) (OtherActor :type Actor%20Object%20Reference) (OtherComp :type Primitive%20Component%20Object%20Reference) (OtherBodyIndex :type Integer) (bFromSweep :type Boolean) (SweepResult :type Hit%20Result%20Structure%20%28by%20ref%29))
  (Variables|Default|SetisInCollision true)
  (Variables|/Game/ThirdPersonBP/Blueprints/ThirdPersonCharacter.ThirdPersonCharacter_C|Setlos1 (stale EventBeginPlay _asthird_person_character) (Math|Random|RandomInteger 10))
  (Variables|/Game/ThirdPersonBP/Blueprints/ThirdPersonCharacter.ThirdPersonCharacter_C|Setlos2 (stale EventBeginPlay _asthird_person_character) (Math|Random|RandomInteger 10))
  (Variables|/Game/ThirdPersonBP/Blueprints/ThirdPersonCharacter.ThirdPersonCharacter_C|Setlos3 (stale EventBeginPlay _asthird_person_character) (Math|Random|RandomInteger 4))
  (Variables|/Game/ThirdPersonBP/Blueprints/ThirdPersonCharacter.ThirdPersonCharacter_C|Setlos4 (stale EventBeginPlay _asthird_person_character) (Math|Random|RandomInteger 10))
  (UserInterface|Viewport|AddtoViewport (stale EventBeginPlay _returnvalue_3) 0)
  (Variables|/Game/content/postac/reginaAnimationBP.reginaAnimationBP_C|SetisInNagrobekCollider (stale EventBeginPlay _asregina_animation_bp) true))

(event OnComponentEndOverlap(collision)
  (params (OverlappedComponent :type Primitive%20Component%20Object%20Reference) (OtherActor :type Actor%20Object%20Reference) (OtherComp :type Primitive%20Component%20Object%20Reference) (OtherBodyIndex :type Integer))
  (Variables|Default|SetisInCollision false)
  (Variables|/Game/content/postac/reginaAnimationBP.reginaAnimationBP_C|SetisInNagrobekCollider (stale EventBeginPlay _asregina_animation_bp) false)
  (Widget|RemovefromParent (stale EventBeginPlay _returnvalue_3)))

(event EventBeginPlay
  (bind _returnvalue (Math|Random|RandomInteger 30))
  (bind _nagrobek06 (Variables|Default|Getnagrobek06))
  (bind _nagrobek04 (Variables|Default|Getnagrobek04))
  (bind _nagrobek03 (Variables|Default|Getnagrobek03))
  (bind _nagrobek02 (Variables|Default|Getnagrobek02))
  (bind _nagrobek01 (Variables|Default|Getnagrobek01))
  (bind _nagrobek05 (Variables|Default|Getnagrobek05))
  (bind _swieczka01 (Variables|Default|Getswieczka01))
  (bind _swieczka09 (Variables|Default|Getswieczka09))
  (bind _returnvalue_2 (>= _returnvalue 15))
  (bind _returnvalue_3 (UserInterface|CreateWidget "/Game/UL/ul_nagrobki.ul_nagrobki_C"))
  (bind _asthird_person_character (Utilities|Casting|CastToThirdPersonCharacter (Game|Player|GetPlayerPawn 0)))
  (bind _asregina_animation_bp (Utilities|Casting|CastToreginaAnimationBP (Components|SkeletalMesh|GetAnimInstance (Variables|/Script/Engine.Character|GetMesh _asthird_person_character))))
  (Variables|Default|SetukladSwieczek (Math|Random|RandomInteger 5))
  (switch int (Math|Random|RandomInteger 6)
    (:0
      (Components|DestroyComponent _nagrobek02)
      (if _returnvalue_2
        (Rendering|Material|SetMaterial _nagrobek01 0 "/Game/Materialy/Materialy/M_nagrobki/M_nagrobek01_01_Inst.M_nagrobek01_01_Inst")
        (else
          (Rendering|Material|SetMaterial _nagrobek01 0 "/Game/Materialy/Materialy/M_nagrobki/M_nagrobek01_02_Inst.M_nagrobek01_02_Inst")))
      (switch int (Variables|Default|GetukladSwieczek) :!label _label
        (:0
          (Rendering|SetVisibility (Variables|Default|Getswieczka01) true false))
        (:1
          (Rendering|SetVisibility (Variables|Default|Getswieczka05) true false))
        (:2
          (Rendering|SetVisibility (Variables|Default|GetP_swieca6) true false))
        (:3
          (Rendering|SetVisibility (Variables|Default|Getswieczka02) true false))
        (:4
          (Rendering|SetVisibility (Variables|Default|Getswieczka06) true false))))
    (:1
      (Components|DestroyComponent _nagrobek01)
      (if _returnvalue_2
        (Rendering|Material|SetMaterial _nagrobek02 0 "/Game/Materialy/Materialy/M_nagrobki/M_nagrobek02_01_Inst.M_nagrobek02_01_Inst")
        (goto _label)
        (else
          (Rendering|Material|SetMaterial _nagrobek02 0 "/Game/Materialy/Materialy/M_nagrobki/M_nagrobek02_02_Inst.M_nagrobek02_02_Inst")
          (goto _label))))
    (:2
      (Components|DestroyComponent _nagrobek02)
      (if _returnvalue_2
        (Rendering|Material|SetMaterial _nagrobek03 0 "/Game/Materialy/Materialy/M_nagrobki/M_nagrobek03_01_Inst.M_nagrobek03_01_Inst")
        (else
          (Rendering|Material|SetMaterial _nagrobek03 0 "/Game/Materialy/Materialy/M_nagrobki/M_nagrobek03_02_Inst.M_nagrobek03_02_Inst")))
      (switch int (Variables|Default|GetukladSwieczek)
        (:0
          (Rendering|SetVisibility _swieczka01 true false))
        (:1
          (Rendering|SetVisibility (Variables|Default|GetP_swieca9) true false))
        (:2
          (Rendering|SetVisibility (Variables|Default|GetP_swieca8) true false))
        (:3
          (Rendering|SetVisibility (Variables|Default|Getswieczka04) true false))
        (:4
          (Rendering|SetVisibility _swieczka01 true false))))
    (:3
      (Components|DestroyComponent _nagrobek02)
      (if _returnvalue_2
        (Rendering|Material|SetMaterial _nagrobek04 0 "/Game/Materialy/Materialy/M_nagrobki/M_nagrobek04_01_Inst.M_nagrobek04_01_Inst")
        (else
          (Rendering|Material|SetMaterial _nagrobek04 0 "/Game/Materialy/Materialy/M_nagrobki/M_nagrobek04_02_Inst.M_nagrobek04_02_Inst")))
      (switch int (Variables|Default|GetukladSwieczek)
        (:0
          (Rendering|SetVisibility (Variables|Default|Getswieczka12) true false))
        (:1
          (Rendering|SetVisibility _swieczka09 true false))
        (:2
          (Rendering|SetVisibility _swieczka09 true false))
        (:3
          (Rendering|SetVisibility (Variables|Default|Getswieczka01) true false))
        (:4
          (Rendering|SetVisibility (Variables|Default|Getswieczka06) true false))))
    (:4
      (Components|DestroyComponent _nagrobek02)
      (if _returnvalue_2
        (Rendering|Material|SetMaterial _nagrobek05 0 "/Game/Materialy/Materialy/M_nagrobki/M_nagrobek05_01_Inst.M_nagrobek05_01_Inst")
        (else
          (Rendering|Material|SetMaterial _nagrobek05 0 "/Game/Materialy/Materialy/M_nagrobki/M_nagrobek05_02_Inst.M_nagrobek05_02_Inst")))
      (switch int (Variables|Default|GetukladSwieczek) :!label _label_2))
    (:5
      (Components|DestroyComponent _nagrobek05)
      (if _returnvalue_2
        (Rendering|Material|SetMaterial _nagrobek06 0 "/Game/Materialy/Materialy/M_granit_02.M_granit_02")
        (goto _label_2)
        (else
          (Rendering|Material|SetMaterial _nagrobek06 0 "/Game/Materialy/Materialy/M_granit_02_Inst.M_granit_02_Inst")
          (goto _label_2))))))

(event EventTick
  (params (DeltaSeconds :type Float%20%28single-precision%29))
  (if (Variables|Default|GetisInCollision)
    (if (Variables|/Game/ThirdPersonBP/Blueprints/ThirdPersonCharacter.ThirdPersonCharacter_C|GetisPPresed (stale EventBeginPlay _asthird_person_character))
      (Variables|/Game/ThirdPersonBP/Blueprints/ThirdPersonCharacter.ThirdPersonCharacter_C|SetisPPresed (stale EventBeginPlay _asthird_person_character) false))))

(fn ConstructionScript)