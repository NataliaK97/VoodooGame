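; Ring pickup actor that starts hidden and appears once the player character's CzyPierscienWidoczny flag is set.
; Box overlap records whether something is in range and sets IsInMuszelkaColider on the player's reginaAnimationBP, without checking which actor overlaps.
; Tick polls for visibility and the character's IsPPresed flag while in range.
; After a short delay, it flags the character as holding the ring with the code displayed, then destroys both components.
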(event OnComponentBeginOverlap(Box)
  (params (OverlappedComponent :type Primitive%20Component%20Object%20Reference) (OtherActor :type Actor%20Object%20Reference) (OtherComp :type Primitive%20Component%20Object%20Reference) (OtherBodyIndex :type Integer) (bFromSweep :type Boolean) (SweepResult :type Hit%20Result%20Structure%20%28by%20ref%29))
  (Variables|Default|SetisInCollider true)
  (bind _asthird_person_character (Utilities|Casting|CastToThirdPersonCharacter (Game|Player|GetPlayerPawn 0)))
  (bind _asregina_animation_bp (Utilities|Casting|CastToreginaAnimationBP (Components|SkeletalMesh|GetAnimInstance (Variables|/Script/Engine.Character|GetMesh _asthird_person_character))))
  (Variables|/Game/content/postac/reginaAnimationBP.reginaAnimationBP_C|SetisInMuszelkaColider _asregina_animation_bp true))

(event OnComponentEndOverlap(Box)
  (params (OverlappedComponent :type Primitive%20Component%20Object%20Reference) (OtherActor :type Actor%20Object%20Reference) (OtherComp :type Primitive%20Component%20Object%20Reference) (OtherBodyIndex :type Integer))
  (Variables|Default|SetisInCollider false)
  (Variables|/Game/content/postac/reginaAnimationBP.reginaAnimationBP_C|SetisInMuszelkaColider (stale OnComponentBeginOverlap(Box) _asregina_animation_bp) false))

(event EventBeginPlay
  (bind _asthird_person_character (Utilities|Casting|CastToThirdPersonCharacter (Game|Player|GetPlayerPawn 0)))
  (Rendering|SetVisibility (Variables|Default|Getpierscionek) false false))

(event Collision|EventActorBeginOverlap
  (params (OtherActor :type Actor%20Object%20Reference)))

(event EventTick
  (params (DeltaSeconds :type Float%20%28single-precision%29))
  (if (Variables|/Game/ThirdPersonBP/Blueprints/ThirdPersonCharacter.ThirdPersonCharacter_C|GetczyPierscienWidoczny (stale EventBeginPlay _asthird_person_character))
    (Rendering|SetVisibility (Variables|Default|Getpierscionek) true false)
    (if (Variables|Default|GetisInCollider)
      (if (Variables|/Game/ThirdPersonBP/Blueprints/ThirdPersonCharacter.ThirdPersonCharacter_C|GetisPPresed (stale EventBeginPlay _asthird_person_character))
        (Utilities|FlowControl|Delay 2.4)
        (Variables|/Game/ThirdPersonBP/Blueprints/ThirdPersonCharacter.ThirdPersonCharacter_C|SetczyMaPierscien (stale EventBeginPlay _asthird_person_character) true)
        (Variables|/Game/ThirdPersonBP/Blueprints/ThirdPersonCharacter.ThirdPersonCharacter_C|SetKodWyswietlony (stale EventBeginPlay _asthird_person_character) true)
        (Components|DestroyComponent (Variables|Default|GetBox))))))

(fn ConstructionScript)