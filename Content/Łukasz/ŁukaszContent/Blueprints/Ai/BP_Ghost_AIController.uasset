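; AI controller for the ghost enemy that sets up its blackboard and starts its behavior tree on BeginPlay.
; It loads BB_Ghost and stores the pawn's starting position as HomeLocation.
; It copies PatrolLocation from the controlled BP_Ghost_Character into the blackboard, then runs BT_Ghots.
; If the pawn is not a BP_Ghost_Character, setup stops before the tree runs.
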(event EventBeginPlay
  (bind _returnvalue (Pawn|GetControlledPawn))
  (Class|AIController|UseBlackboard "/Game/Łukasz/ŁukaszContent/Blueprints/Ai/BB_Ghost.BB_Ghost")
  (AI|Components|Blackboard|SetValueasVector (AI|GetBlackboard self) (Variables|Default|GetHomeLocation) (Transformation|GetActorLocation _returnvalue))
  (bind _asbp_ghost_character (Utilities|Casting|CastToBP_Ghost_Character _returnvalue))
  (AI|Components|Blackboard|SetValueasVector (AI|GetBlackboard self) (Variables|Default|GetPatrolLocation) (Variables|/Game/Łukasz/ŁukaszContent/Blueprints/Ai/BP_Ghost_Character.BP_Ghost_Character_C|GetPatrolLocation _asbp_ghost_character))
  (AI|RunBehaviorTree "/Game/Łukasz/ŁukaszContent/Blueprints/Ai/BT_GHots.BT_Ghots"))

(fn ConstructionScript)