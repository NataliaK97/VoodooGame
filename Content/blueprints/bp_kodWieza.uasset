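; Trigger actor that shows the tower code widget (Ul_kodWieza) while its ColliderKod volume is overlapped.
; Begin overlap caches the player pawn as ThirdPersonCharacter, shows the mouse cursor and adds a new widget to the viewport, without checking the overlapping actor.
; End overlap hides the cursor, removes the widget and destroys the collider if the character's UsunKoliderKod flag is set.
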(event OnComponentBeginOverlap(colliderKod)
  (params (OverlappedComponent :type Primitive%20Component%20Object%20Reference) (OtherActor :type Actor%20Object%20Reference) (OtherComp :type Primitive%20Component%20Object%20Reference) (OtherBodyIndex :type Integer) (bFromSweep :type Boolean) (SweepResult :type Hit%20Result%20Structure%20%28by%20ref%29))
  (bind _asthird_person_character (Utilities|Casting|CastToThirdPersonCharacter (Game|Player|GetPlayerPawn 0)))
  (Variables|/Script/Engine.PlayerController|SetbShowMouseCursor (Game|GetPlayerController 0) true)
  (bind _returnvalue (UserInterface|CreateWidget "/Game/UL/ul_kodWieza.ul_kodWieza_C"))
  (UserInterface|Viewport|AddtoViewport _returnvalue 0))

(event OnComponentEndOverlap(colliderKod)
  (params (OverlappedComponent :type Primitive%20Component%20Object%20Reference) (OtherActor :type Actor%20Object%20Reference) (OtherComp :type Primitive%20Component%20Object%20Reference) (OtherBodyIndex :type Integer))
  (Variables|/Script/Engine.PlayerController|SetbShowMouseCursor (Game|GetPlayerController 0) false)
  (Widget|RemovefromParent (stale OnComponentBeginOverlap(colliderKod) _returnvalue))
  (if (Variables|/Game/ThirdPersonBP/Blueprints/ThirdPersonCharacter.ThirdPersonCharacter_C|GetusunKoliderKod (stale OnComponentBeginOverlap(colliderKod) _asthird_person_character))
    (Components|DestroyComponent (Variables|Default|GetcolliderKod))))

(event EventBeginPlay)

(event Collision|EventActorBeginOverlap
  (params (OtherActor :type Actor%20Object%20Reference)))

(event EventTick
  (params (DeltaSeconds :type Float%20%28single-precision%29)))

(fn ConstructionScript)