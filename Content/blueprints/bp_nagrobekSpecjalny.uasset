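; Special gravestone actor (nagrobek specjalny) that lets the player trigger the cemetery task display.
; On BeginPlay it keeps one random tombstone mesh, picks one of two materials for it and shows matching candle components.
; Its collision overlap shows a UI widget, flags Regina's anim blueprint, rerolls Los3 and can set the journal code flag.
; While overlapping, Tick polls the character's P-press flag, then sets the task flag after a delay.
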(event OnComponentBeginOverlap(collision)
  (params (OverlappedComponent :type Primitive%20Component%20Object%20Reference) (OtherActor :type Actor%20Object%20Reference) (OtherComp :type Primitive%20Component%20Object%20Reference) (OtherBodyIndex :type Integer) (bFromSweep :type Boolean) (SweepResult :type Hit%20Result%20Structure%20%28by%20ref%29))
  (bind _returnvalue (UserInterface|CreateWidget "/Game/UL/ul_nagrobekSpecjalny.ul_nagrobekSpecjalny_C"))
  (Variables|/Game/ThirdPersonBP/Blueprints/ThirdPersonCharacter.ThirdPersonCharacter_C|Setlos3 (stale EventBeginPlay _asthird_person_character) (Math|Random|RandomInteger 4))
  (Variables|Default|SetisInCollision true)
  (UserInterface|Viewport|AddtoViewport _returnvalue 0)
  (Variables|/Game/content/postac/reginaAnimationBP.reginaAnimationBP_C|SetisInNagrobekCollider (stale EventBeginPlay _asregina_animation_bp) true)
  (if (Variables|/Game/ThirdPersonBP/Blueprints/ThirdPersonCharacter.ThirdPersonCharacter_C|GetKodWyswietlony (stale EventBeginPlay _asthird_person_character))
    (Variables|/Game/ThirdPersonBP/Blueprints/ThirdPersonCharacter.ThirdPersonCharacter_C|SetKodWDzienniku (stale EventBeginPlay _asthird_person_character) true)))

(event OnComponentEndOverlap(collision)
  (params (OverlappedComponent :type Primitive%20Component%20Object%20Reference) (OtherActor :type Actor%20Object%20Reference) (OtherComp :type Primitive%20Component%20Object%20Reference) (OtherBodyIndex :type Integer))
  (Variables|Default|SetisInCollision false)
  (Variables|/Game/content/postac/reginaAnimationBP.reginaAnimationBP_C|SetisInNagrobekCollider (stale EventBeginPlay _asregina_animation_bp) false)
  (Widget|RemovefromParent (stale OnComponentBeginOverlap(collision) _returnvalue)))

(event EventBeginPlay
  (bind _returnvalue (Math|Random|RandomInteger 30))
  (bind _nagrobek01 (Variables|Default|Getnagrobek01))
  (bind _nagrobek02 (Variables|Default|Getnagrobek02))
  (bind _nagrobek03 (Variables|Default|Getnagrobek03))
  (bind _nagrobek012 (Variables|Default|Getnagrobek012))
  (bind _returnvalue_2 (>= _returnvalue 15))
  (bind _asthird_person_character (Utilities|Casting|CastToThirdPersonCharacter (Game|Player|GetPlayerPawn 0)))
  (bind _asregina_animation_bp (Utilities|Casting|CastToreginaAnimationBP (Components|SkeletalMesh|GetAnimInstance (Variables|/Script/Engine.Character|GetMesh _asthird_person_character))))
  (switch int (Math|Random|RandomInteger 4)
    (:0
      (Components|DestroyComponent _nagrobek02)
      (if _returnvalue_2
        (Rendering|Material|SetMaterial _nagrobek01 0 "/Game/Materialy/Materialy/M_nagrobki/M_nagrobek01_01_Inst.M_nagrobek01_01_Inst")
        (else
          (Rendering|Material|SetMaterial _nagrobek01 0 "/Game/Materialy/Materialy/M_nagrobki/M_nagrobek01_02_Inst.M_nagrobek01_02_Inst")))
      (Rendering|SetVisibility (Variables|Default|GetP_swieca8) true false :!label _label))
    (:1
      (Components|DestroyComponent _nagrobek01)
      (if _returnvalue_2
        (Rendering|Material|SetMaterial _nagrobek02 0 "/Game/Materialy/Materialy/M_nagrobki/M_nagrobek02_01_Inst.M_nagrobek02_01_Inst")
        (goto _label)
        (else
          (Rendering|Material|SetMaterial _nagrobek02 0 "/Game/Materialy/Materialy/M_nagrobki/M_nagrobek02_02_Inst.M_nagrobek02_02_Inst")
          (goto _label))))
    (:2
      (Components|DestroyComponent _nagrobek01)
      (if _returnvalue_2
        (Rendering|Material|SetMaterial _nagrobek03 0 "/Game/Materialy/Materialy/M_nagrobki/M_nagrobek03_01_Inst.M_nagrobek03_01_Inst")
        (goto _label)
        (else
          (Rendering|Material|SetMaterial _nagrobek03 0 "/Game/Materialy/Materialy/M_nagrobki/M_nagrobek03_02_Inst.M_nagrobek03_02_Inst")
          (goto _label))))
    (:3
      (Components|DestroyComponent _nagrobek03 :!label _label_2)
      (if _returnvalue_2
        (Rendering|Material|SetMaterial _nagrobek012 0 "/Game/Materialy/Materialy/M_nagrobki/M_nagrobek04_01_Inst.M_nagrobek04_01_Inst")
        (else
          (Rendering|Material|SetMaterial _nagrobek012 0 "/Game/Materialy/Materialy/M_nagrobki/M_nagrobek04_02_Inst.M_nagrobek04_02_Inst")))
      (Rendering|SetVisibility (Variables|Default|Getswieczka011) true false))
    (:4
      (goto _label_2))))

(event EventTick
  (params (DeltaSeconds :type Float%20%28single-precision%29))
  (if (Variables|Default|GetisInCollision)
    (if (Variables|/Game/ThirdPersonBP/Blueprints/ThirdPersonCharacter.ThirdPersonCharacter_C|GetisPPresed (stale EventBeginPlay _asthird_person_character))
      (Variables|/Game/ThirdPersonBP/Blueprints/ThirdPersonCharacter.ThirdPersonCharacter_C|SetisPPresed (stale EventBeginPlay _asthird_person_character) false)
      (Utilities|FlowControl|Delay 2.2)
      (Variables|/Game/ThirdPersonBP/Blueprints/ThirdPersonCharacter.ThirdPersonCharacter_C|SetWyswietlZadanieCmentarz (stale EventBeginPlay _asthird_person_character) true))))

(fn ConstructionScript)