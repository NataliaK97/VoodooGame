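; Behavior tree service that detects nearby visible targets for the ghost AI and writes them to the blackboard.
; Each tick it sphere-traces around the pawn, then line-traces on the Camera channel to each hit to confirm line of sight, ignoring other ghosts.
; Visible hits set TargetToFollow and TargetLocation; failed checks clear only TargetToFollow, keeping the last seen location.
; The last hit evaluated decides the target.
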(event EventTick
  (params (OwnerActor :type Actor%20Object%20Reference) (DeltaSeconds :type Float%20%28single-precision%29))
  ;[1 1 1] Is AICONTROLLER_REF set?
  (if (!= (Variables|Default|GetAICOntroller_Ref) 0)
    _
    (else
      (bind _asbp_ghost_aicontroller (Utilities|Casting|CastToBP_Ghost_AIController OwnerActor))
      (Variables|Default|SetAICOntroller_Ref _asbp_ghost_aicontroller)))
  (bind _outactors (Actor|GetAllActorsOfClass "/Game/Łukasz/ŁukaszContent/Blueprints/Ai/BP_Ghost_Character.BP_Ghost_Character_C"))
  (Variables|Default|SetMyLocation (Transformation|GetActorLocation (Pawn|GetControlledPawn (Variables|Default|GetAICOntroller_Ref))))
  (bind (_outhits _returnvalue) (Collision|MultiSphereTraceForObjects (Transformation|GetActorLocation (Pawn|GetControlledPawn (Variables|Default|GetAICOntroller_Ref))) (+ (Transformation|GetActorLocation (Pawn|GetControlledPawn (Variables|Default|GetAICOntroller_Ref))) "0, 0,15.000000") 1.5e+03 (Variables|Default|GetDesiredObjectTypes) false _outactors "None"))
  (if _returnvalue
    (for _array_element _outhits
      (bind _outhit (Collision|LineTraceByChannel (Variables|Default|GetMyLocation) (Transformation|GetActorLocation (.HitActor (Collision|BreakHitResult _array_element))) "TraceTypeQuery2" false _outactors "None"))
      (if (== (.HitActor (Collision|BreakHitResult _outhit)) (.HitActor (Collision|BreakHitResult _array_element)))
        (Class|BTFunctionLibrary|SetBlackboardValueasObject (Variables|Default|GetTargetToFollow) (.HitActor (Collision|BreakHitResult _outhit)))
        (AI|BehaviorTree|SetBlackboardValueasVector (Variables|Default|GetTargetLocation) (Transformation|GetActorLocation (.HitActor (Collision|BreakHitResult _outhit))))
        (else
          (Class|BTFunctionLibrary|SetBlackboardValueasObject (Variables|Default|GetTargetToFollow)))))
    (else
      (Class|BTFunctionLibrary|SetBlackboardValueasObject (Variables|Default|GetTargetToFollow)))))