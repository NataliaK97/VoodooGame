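; Ocean actor Blueprint that flags the player and shows an ocean UI while either of two warning volumes is overlapped.
; BeginPlay caches the ThirdPersonCharacter, whose Ocean1 or Ocean2 boolean is toggled by the Warning and Warning2 overlap events.
; Both begin events share creation of a Ul_ocean widget, and both end events remove the last one created.
; Overlaps do not check which actor triggered them.
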(event OnComponentBeginOverlap(warning)
  (params (OverlappedComponent :type Primitive%20Component%20Object%20Reference) (OtherActor :type Actor%20Object%20Reference) (OtherComp :type Primitive%20Component%20Object%20Reference) (OtherBodyIndex :type Integer) (bFromSweep :type Boolean) (SweepResult :type Hit%20Result%20Structure%20%28by%20ref%29))
  (Variables|/Game/ThirdPersonBP/Blueprints/ThirdPersonCharacter.ThirdPersonCharacter_C|SetOcean_1 (stale EventBeginPlay _asthird_person_character) true)
  (bind _returnvalue (UserInterface|CreateWidget "/Game/UL/ul_ocean.ul_ocean_C"))
  (UserInterface|Viewport|AddtoViewport _returnvalue 0))

(event OnComponentEndOverlap(warning2)
  (params (OverlappedComponent :type Primitive%20Component%20Object%20Reference) (OtherActor :type Actor%20Object%20Reference) (OtherComp :type Primitive%20Component%20Object%20Reference) (OtherBodyIndex :type Integer))
  (Variables|/Game/ThirdPersonBP/Blueprints/ThirdPersonCharacter.ThirdPersonCharacter_C|SetOcean_2 (stale EventBeginPlay _asthird_person_character) false)
  (Widget|RemovefromParent (stale OnComponentBeginOverlap(warning) _returnvalue)))

(event OnComponentEndOverlap(warning)
  (params (OverlappedComponent :type Primitive%20Component%20Object%20Reference) (OtherActor :type Actor%20Object%20Reference) (OtherComp :type Primitive%20Component%20Object%20Reference) (OtherBodyIndex :type Integer))
  (Variables|/Game/ThirdPersonBP/Blueprints/ThirdPersonCharacter.ThirdPersonCharacter_C|SetOcean_1 (stale EventBeginPlay _asthird_person_character) false)
  (Widget|RemovefromParent (stale OnComponentBeginOverlap(warning) _returnvalue)))

(event OnComponentBeginOverlap(warning2)
  (params (OverlappedComponent :type Primitive%20Component%20Object%20Reference) (OtherActor :type Actor%20Object%20Reference) (OtherComp :type Primitive%20Component%20Object%20Reference) (OtherBodyIndex :type Integer) (bFromSweep :type Boolean) (SweepResult :type Hit%20Result%20Structure%20%28by%20ref%29))
  (Variables|/Game/ThirdPersonBP/Blueprints/ThirdPersonCharacter.ThirdPersonCharacter_C|SetOcean_2 (stale EventBeginPlay _asthird_person_character) true)
  (bind _returnvalue (UserInterface|CreateWidget "/Game/UL/ul_ocean.ul_ocean_C"))
  (UserInterface|Viewport|AddtoViewport _returnvalue 0))

(event EventBeginPlay
  (bind _asthird_person_character (Utilities|Casting|CastToThirdPersonCharacter (Game|Player|GetPlayerPawn 0))))

(event EventTick
  (params (DeltaSeconds :type Float%20%28single-precision%29)))

(fn ConstructionScript)