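; Clown actor that reacts when something enters or leaves its Box trigger, switching animations and showing a UI widget.
; The Ul_clown widget is created at BeginPlay; each overlap increments its IleRazy counter and adds it to the viewport.
; Flags on the bp_ClownAmination AnimInstance make the clown stand, then laugh after a short delay.
; Leaving removes the widget, clears those flags and sets CanSit.
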(event OnComponentBeginOverlap(Box)
  (params (OverlappedComponent :type Primitive%20Component%20Object%20Reference) (OtherActor :type Actor%20Object%20Reference) (OtherComp :type Primitive%20Component%20Object%20Reference) (OtherBodyIndex :type Integer) (bFromSweep :type Boolean) (SweepResult :type Hit%20Result%20Structure%20%28by%20ref%29))
  (Variables|/Game/UL/ul_clown.ul_clown_C|Setile%20razy (stale EventBeginPlay _returnvalue) (+ (Variables|/Game/UL/ul_clown.ul_clown_C|Getile%20razy (stale EventBeginPlay _returnvalue)) 1))
  (UserInterface|Viewport|AddtoViewport (stale EventBeginPlay _returnvalue) 0)
  (bind _asbp_clown_amination (Utilities|Casting|CastTobp_ClownAmination (Components|SkeletalMesh|GetAnimInstance (Variables|Default|Getclown))))
  (Variables|/Game/content/postac/clown/bp_ClownAmination.bp_ClownAmination_C|SetcanStand _asbp_clown_amination true)
  (Utilities|FlowControl|Delay 2.0)
  (Variables|/Game/content/postac/clown/bp_ClownAmination.bp_ClownAmination_C|SetcanLaught _asbp_clown_amination true))

(event OnComponentEndOverlap(Box)
  (params (OverlappedComponent :type Primitive%20Component%20Object%20Reference) (OtherActor :type Actor%20Object%20Reference) (OtherComp :type Primitive%20Component%20Object%20Reference) (OtherBodyIndex :type Integer))
  (Widget|RemovefromParent (stale EventBeginPlay _returnvalue))
  (Variables|/Game/content/postac/clown/bp_ClownAmination.bp_ClownAmination_C|SetcanStand (stale OnComponentBeginOverlap(Box) _asbp_clown_amination) false)
  (Variables|/Game/content/postac/clown/bp_ClownAmination.bp_ClownAmination_C|SetcanLaught (stale OnComponentBeginOverlap(Box) _asbp_clown_amination) false)
  (Variables|/Game/content/postac/clown/bp_ClownAmination.bp_ClownAmination_C|SetcanSit (stale OnComponentBeginOverlap(Box) _asbp_clown_amination) true))

(event EventBeginPlay
  (bind _returnvalue (UserInterface|CreateWidget "/Game/UL/ul_clown.ul_clown_C"))
  (Variables|/Game/UL/ul_clown.ul_clown_C|Setile%20razy _returnvalue 0))

(event Collision|EventActorBeginOverlap
  (params (OtherActor :type Actor%20Object%20Reference)))

(event EventTick
  (params (DeltaSeconds :type Float%20%28single-precision%29)))

(fn ConstructionScript)