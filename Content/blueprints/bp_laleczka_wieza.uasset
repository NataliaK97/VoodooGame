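; Collectible voodoo doll pickup (named for a tower) that adds to the player character's doll count, IloscLaleczek.
; Overlap events on its collider set a flag without checking the other actor, and Tick polls that flag.
; When the flag is set, Tick increments the count on the cached ThirdPersonCharacter and destroys the collider and doll components.
; A looping Delay then steps the spotlight's intensity down to zero before destroying it.
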(event OnComponentBeginOverlap(ColliderLaleczki)
  (params (OverlappedComponent :type Primitive%20Component%20Object%20Reference) (OtherActor :type Actor%20Object%20Reference) (OtherComp :type Primitive%20Component%20Object%20Reference) (OtherBodyIndex :type Integer) (bFromSweep :type Boolean) (SweepResult :type Hit%20Result%20Structure%20%28by%20ref%29))
  (Variables|Default|SetisInCollider true))

(event OnComponentEndOverlap(ColliderLaleczki)
  (params (OverlappedComponent :type Primitive%20Component%20Object%20Reference) (OtherActor :type Actor%20Object%20Reference) (OtherComp :type Primitive%20Component%20Object%20Reference) (OtherBodyIndex :type Integer))
  (Variables|Default|SetisInCollider false))

(event EventBeginPlay
  (bind _asthird_person_character (Utilities|Casting|CastToThirdPersonCharacter (Game|Player|GetPlayerPawn 0))))

(event Collision|EventActorBeginOverlap
  (params (OtherActor :type Actor%20Object%20Reference)))

(event EventTick
  (params (DeltaSeconds :type Float%20%28single-precision%29))
  (bind _spotlight (Variables|Default|GetSpotLight))
  (bind _intensity (Variables|/Script/Engine.LightComponentBase|GetIntensity _spotlight))
  (if (Variables|Default|GetisInCollider)
    (Variables|/Game/ThirdPersonBP/Blueprints/ThirdPersonCharacter.ThirdPersonCharacter_C|SetiloscLaleczek (stale EventBeginPlay _asthird_person_character) (+ (Variables|/Game/ThirdPersonBP/Blueprints/ThirdPersonCharacter.ThirdPersonCharacter_C|GetiloscLaleczek (stale EventBeginPlay _asthird_person_character)) 1))
    (Components|DestroyComponent (Variables|Default|GetColliderLaleczki))
    (Rendering|Components|Light|SetIntensity _spotlight (- _intensity 5.0) :!label _label)
    (Utilities|FlowControl|Delay 0.1)
    (if (<= _intensity 0.0)
      (Components|DestroyComponent (Variables|Default|GetSpotLight))
      (else
        (goto _label)))))

(fn ConstructionScript)