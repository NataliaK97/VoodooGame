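; Holy water (WodaSw) pickup that the player character can drink up to three times, as counted on the character.
; Box overlap flags the player as in range, both locally and in the Regina animation Blueprint.
; While in range, Tick consumes the character's P-press flag, sets its drunk state, removes a water mesh after a delay, then clears that state after a longer delay.
; Once the limit is reached, Tick destroys the box.
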(event OnComponentBeginOverlap(Box)
  (params (OverlappedComponent :type Primitive%20Component%20Object%20Reference) (OtherActor :type Actor%20Object%20Reference) (OtherComp :type Primitive%20Component%20Object%20Reference) (OtherBodyIndex :type Integer) (bFromSweep :type Boolean) (SweepResult :type Hit%20Result%20Structure%20%28by%20ref%29))
  (Variables|Default|SetisInColliderr true)
  (bind _asthird_person_character (Utilities|Casting|CastToThirdPersonCharacter (Game|Player|GetPlayerPawn 0)))
  (bind _asregina_animation_bp (Utilities|Casting|CastToreginaAnimationBP (Components|SkeletalMesh|GetAnimInstance (Variables|/Script/Engine.Character|GetMesh _asthird_person_character))))
  (Variables|/Game/content/postac/reginaAnimationBP.reginaAnimationBP_C|SetisInWodaSwColider _asregina_animation_bp true))

(event OnComponentEndOverlap(Box)
  (params (OverlappedComponent :type Primitive%20Component%20Object%20Reference) (OtherActor :type Actor%20Object%20Reference) (OtherComp :type Primitive%20Component%20Object%20Reference) (OtherBodyIndex :type Integer))
  (Variables|Default|SetisInColliderr false)
  (Variables|/Game/content/postac/reginaAnimationBP.reginaAnimationBP_C|SetisInWodaSwColider (stale OnComponentBeginOverlap(Box) _asregina_animation_bp) false))

(event EventBeginPlay)

(event Collision|EventActorBeginOverlap
  (params (OtherActor :type Actor%20Object%20Reference)))

(event EventTick
  (params (DeltaSeconds :type Float%20%28single-precision%29))
  (if (Variables|Default|GetisInColliderr)
    (bind _asthird_person_character (Utilities|Casting|CastToThirdPersonCharacter (Game|Player|GetPlayerPawn 0)))
    (if (<= (Variables|/Game/ThirdPersonBP/Blueprints/ThirdPersonCharacter.ThirdPersonCharacter_C|GetileWypitejWody _asthird_person_character) 2)
      (if (Variables|/Game/ThirdPersonBP/Blueprints/ThirdPersonCharacter.ThirdPersonCharacter_C|GetisPPresed _asthird_person_character)
        (Variables|/Game/ThirdPersonBP/Blueprints/ThirdPersonCharacter.ThirdPersonCharacter_C|SetisPPresed _asthird_person_character false)
        (Variables|/Game/ThirdPersonBP/Blueprints/ThirdPersonCharacter.ThirdPersonCharacter_C|SetileWypitejWody _asthird_person_character (+ (Variables|/Game/ThirdPersonBP/Blueprints/ThirdPersonCharacter.ThirdPersonCharacter_C|GetileWypitejWody _asthird_person_character) 1))
        (Variables|/Game/ThirdPersonBP/Blueprints/ThirdPersonCharacter.ThirdPersonCharacter_C|SetczyWypitaWoda _asthird_person_character true)
        (Utilities|FlowControl|Delay 1.5)
        (switch int (Variables|/Game/ThirdPersonBP/Blueprints/ThirdPersonCharacter.ThirdPersonCharacter_C|GetileWypitejWody _asthird_person_character)
          (:0
            _)
          (:1
            (Components|DestroyComponent (Variables|Default|GetwodaSw_woda003)))
          (:2
            (Components|DestroyComponent (Variables|Default|GetwodaSw_woda002)))
          (:3
            (Components|DestroyComponent (Variables|Default|GetwodaSw_woda001))))
        (Utilities|FlowControl|Delay 2e+01)
        (Variables|/Game/ThirdPersonBP/Blueprints/ThirdPersonCharacter.ThirdPersonCharacter_C|SetczyWypitaWoda _asthird_person_character false))
      (else
        (Components|DestroyComponent (Variables|Default|GetBox))))))

(fn ConstructionScript)