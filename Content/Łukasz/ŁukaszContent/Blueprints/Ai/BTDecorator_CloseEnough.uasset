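; BTDecorator_CloseEnough is a behavior tree decorator that gates a branch on the distance between a ghost AI and its follow target.
; It casts the owner to BP_Ghost_AIController, then measures from the controlled pawn to the actor in the TargetToFollow blackboard key.
; Despite its name, the condition passes when that distance is at least AcceptableDistance, meaning the ghost is not yet closer than the threshold.
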(fn PerformConditionCheck
  (params (OwnerActor :type Actor%20Object%20Reference))
  (bind _asbp_ghost_aicontroller (Utilities|Casting|CastToBP_Ghost_AIController OwnerActor))
  (Variables|Default|SetAIController_Ref _asbp_ghost_aicontroller)
  (return (>= (Math|Vector|VectorLength (- (Transformation|GetActorLocation (AI|BehaviorTree|GetBlackboardValueasActor (Variables|Default|GetTargetToFollow))) (Transformation|GetActorLocation (Pawn|GetControlledPawn (Variables|Default|GetAIController_Ref))))) (Variables|Default|GetAcceptableDistance))))