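; Glowing firefly actor that counts toward a destruction goal stored on the player's ThirdPersonCharacter.
; Any overlap on its Sphere hides both spheres and the light, increments IleZniszczone, then shows them again after 15 seconds.
; Tick keeps them hidden while the goal is met and the firefly doll is uncollected; a 50-second Delay then resets the counter and restores visibility.
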(event OnComponentBeginOverlap(Sphere)
  (params (OverlappedComponent :type Primitive%20Component%20Object%20Reference) (OtherActor :type Actor%20Object%20Reference) (OtherComp :type Primitive%20Component%20Object%20Reference) (OtherBodyIndex :type Integer) (bFromSweep :type Boolean) (SweepResult :type Hit%20Result%20Structure%20%28by%20ref%29))
  (bind _pointlight (Variables|Default|GetPointLight))
  (Rendering|SetVisibility _pointlight false false)
  (Variables|/Game/ThirdPersonBP/Blueprints/ThirdPersonCharacter.ThirdPersonCharacter_C|SetileZniszczone (stale EventBeginPlay _asthird_person_character) (+ (Variables|/Game/ThirdPersonBP/Blueprints/ThirdPersonCharacter.ThirdPersonCharacter_C|GetileZniszczone (stale EventBeginPlay _asthird_person_character)) 1))
  (Utilities|FlowControl|Delay 15.0)
  (Rendering|SetVisibility _pointlight true false))

(event EventBeginPlay
  (bind _asthird_person_character (Utilities|Casting|CastToThirdPersonCharacter (Game|Player|GetPlayerPawn 0))))

(event Collision|EventActorBeginOverlap
  (params (OtherActor :type Actor%20Object%20Reference)))

(event EventTick
  (params (DeltaSeconds :type Float%20%28single-precision%29))
  (if (and (>= (Variables|/Game/ThirdPersonBP/Blueprints/ThirdPersonCharacter.ThirdPersonCharacter_C|GetileZniszczone (stale EventBeginPlay _asthird_person_character)) (Variables|/Game/ThirdPersonBP/Blueprints/ThirdPersonCharacter.ThirdPersonCharacter_C|GetileSwietlikowZniszczyc (stale EventBeginPlay _asthird_person_character))) (not (Variables|/Game/ThirdPersonBP/Blueprints/ThirdPersonCharacter.ThirdPersonCharacter_C|GetlaleczkaSwietlikiZebrana (stale EventBeginPlay _asthird_person_character))))
    (Rendering|SetVisibility (Variables|Default|GetSphere1) false false)
    (Utilities|FlowControl|Delay 5e+01)
    (Variables|/Game/ThirdPersonBP/Blueprints/ThirdPersonCharacter.ThirdPersonCharacter_C|SetileZniszczone (stale EventBeginPlay _asthird_person_character) 0)
    (Rendering|SetVisibility (Variables|Default|GetPointLight) true false)))

(fn ConstructionScript)