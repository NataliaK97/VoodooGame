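; Voodoo doll pickup that stays hidden until the player has destroyed the required number of fireflies.
; BeginPlay caches the ThirdPersonCharacter and hides the doll and its collider; Tick polls the character's destroyed count against its target to reveal them.
; Collider overlaps set an in-range flag without filtering the actor.
; Once revealed and in range, Tick increments the character's doll count, flags this doll collected and destroys both components.
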(event OnComponentBeginOverlap(ColliderLaleczki)
  (params (OverlappedComponent :type Primitive%20Component%20Object%20Reference) (OtherActor :type Actor%20Object%20Reference) (OtherComp :type Primitive%20Component%20Object%20Reference) (OtherBodyIndex :type Integer) (bFromSweep :type Boolean) (SweepResult :type Hit%20Result%20Structure%20%28by%20ref%29))
  (bind _output_get (Variables|Default|SetisInCollider true)))

(event OnComponentEndOverlap(ColliderLaleczki)
  (params (OverlappedComponent :type Primitive%20Component%20Object%20Reference) (OtherActor :type Actor%20Object%20Reference) (OtherComp :type Primitive%20Component%20Object%20Reference) (OtherBodyIndex :type Integer))
  (Variables|Default|SetisInCollider false))

(event EventBeginPlay
  (bind _asthird_person_character (Utilities|Casting|CastToThirdPersonCharacter (Game|Player|GetPlayerPawn 0)))
  (Rendering|SetVisibility (Variables|Default|GetlaleczkaVoodoo) false false))

(event Collision|EventActorBeginOverlap
  (params (OtherActor :type Actor%20Object%20Reference)))

(event EventTick
  (params (DeltaSeconds :type Float%20%28single-precision%29))
  (if (>= (Variables|/Game/ThirdPersonBP/Blueprints/ThirdPersonCharacter.ThirdPersonCharacter_C|GetileZniszczone (stale EventBeginPlay _asthird_person_character)) (Variables|/Game/ThirdPersonBP/Blueprints/ThirdPersonCharacter.ThirdPersonCharacter_C|GetileSwietlikowZniszczyc (stale EventBeginPlay _asthird_person_character)))
    (Rendering|SetVisibility (Variables|Default|GetlaleczkaVoodoo) true false)
    (if (stale OnComponentBeginOverlap(ColliderLaleczki) _output_get)
      (Variables|/Game/ThirdPersonBP/Blueprints/ThirdPersonCharacter.ThirdPersonCharacter_C|SetiloscLaleczek (stale EventBeginPlay _asthird_person_character) (+ (Variables|/Game/ThirdPersonBP/Blueprints/ThirdPersonCharacter.ThirdPersonCharacter_C|GetiloscLaleczek (stale EventBeginPlay _asthird_person_character)) 1))
      (Variables|/Game/ThirdPersonBP/Blueprints/ThirdPersonCharacter.ThirdPersonCharacter_C|SetlaleczkaSwietlikiZebrana (stale EventBeginPlay _asthird_person_character) true)
      (Components|DestroyComponent (Variables|Default|GetColliderLaleczki)))))

(fn ConstructionScript)